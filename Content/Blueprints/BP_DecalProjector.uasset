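; Decal projector actor that builds a grid of decals in its local XZ plane at construction, apparently for walls.
; A WallDecalConfigurations data table row supplies a flattened lookup array: zero hides a cell, other values select from Materials (1-based, clamped to the last).
; Cells beyond the array get random materials, so they can change whenever construction reruns.
; Helper functions convert grid coordinates to local and world positions, or retrieve the stored decal.
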(event EventBeginPlay)

(event EventActorBeginOverlap
  (params (OtherActor :type Actor%20Object%20Reference)))

(event EventTick
  (params (DeltaSeconds :type Float%20%28single-precision%29)))

(fn ConstructionScript
  (bind _materials (Variables|Default|GetMaterials))
  (bind _spawnamount (Variables|Default|GetspawnAmount))
  (bind _spawnevery (Variables|Default|GetspawnEvery))
  (bind (_x _y) (Utilities|Struct|BreakBP_2DArraysize_t _spawnamount))
  (bind (_x_2 _y_2) (Math|Vector2D|BreakVector2D _spawnevery))
  ;[1 1 1] Initialise Local variables
  (bind _output_get (LocalVariables|SetNumberOfMaterials (Utilities|Array|Length (Variables|Default|GetMaterials))))
  (bind _returnvalue (Utilities|GetDataTableRow "/Game/Data/WallDecalConfigurations.WallDecalConfigurations" (Variables|Default|GetDataTableRow))
    (:then
      (LocalVariables|SetLUTData (.data (Utilities|Struct|BreakWallDecalInstruction _returnvalue))))
    (:RowNotFound
      (LocalVariables|SetLUTData (Utilities|Array|MakeArray (Class|KismetSystemLibrary|MakeLiteralInteger 1)))))
  (if (> _output_get 0)
    (LocalVariables|SetLUTLength (Utilities|Array|Length (LocalVariables|GetLUTData)))
    ;[1 1 1] Clear array of old decals
    (Utilities|Array|Clear (Variables|Default|GetDecals))
    ;[1 1 1] Create new decals
    (for _index (range 0 (- _y 1))
      (for _index_2 (range 0 (- _x 1))
        (bind _returnvalue_2 (AddComponent|AddDecalComponent false (Math|Transform|MakeTransform (Math|Vector|MakeVector (* _index_2 _x_2) 0.0 (* _index _y_2)) (Math|Rotator|MakeRotator 0.0 0.0 (Variables|Default|GetDecalRotation)) "1,1,1.000000")))
        ;[1 1 1] Get material instance
        (if (< (CallFunction|2DArrayIndexto1DIndex _index_2 _index _x) (LocalVariables|GetLUTLength))
          (LocalVariables|Setenable (!= (Utilities|Array|Get(acopy) (LocalVariables|GetLUTData) (CallFunction|2DArrayIndexto1DIndex _index_2 _index _x)) 0))
          (LocalVariables|SetassignMaterial (Utilities|Array|Get(acopy) _materials (- (Math|Integer|Min(Integer) (Utilities|Array|Get(acopy) (LocalVariables|GetLUTData) (CallFunction|2DArrayIndexto1DIndex _index_2 _index _x)) (LocalVariables|GetNumberOfMaterials)) 1)))
          (else
            (LocalVariables|Setenable true)
            (LocalVariables|SetassignMaterial (Utilities|Array|Get(acopy) _materials (Math|Integer|%(Integer) (Math|Random|RandomInteger 255) (LocalVariables|GetNumberOfMaterials))))))
        ;[1 1 1] Assign Decal Parametres
        (Rendering|Components|Decal|SetDecalMaterial _returnvalue_2 (LocalVariables|GetassignMaterial))
        (Transformation|SetWorldScale3D _returnvalue_2 (Variables|Default|GetDecalScale))
        (Rendering|SetVisibility _returnvalue_2 (LocalVariables|Getenable) false)
        ;[1 1 1] Add To decal array
        (Utilities|Array|Add (Variables|Default|GetDecals) _returnvalue_2)))))

(fn 2DArrayIndexto1DIndex
  (params (A :type Integer) (B :type Integer) (TotalA :type Integer))
  (return (+ A (* B TotalA))))

(fn GetDecalPosition
  (params (x :type Integer) (y :type Integer))
  (bind _spawnevery (Variables|Default|GetspawnEvery))
  (bind _defaultsceneroot (Variables|Default|GetDefaultSceneRoot))
  (bind (_x _y) (Math|Vector2D|BreakVector2D _spawnevery))
  (bind _returnvalue (* y _y))
  (bind _returnvalue_2 (* x _x))
  (bind _returnvalue_3 (Math|Vector|MakeVector _returnvalue_2 0.0 _returnvalue))
  (return (+ (Math|Vector|RotateVector (* _returnvalue_3 (Transformation|GetWorldScale _defaultsceneroot)) (Transformation|GetWorldRotation _defaultsceneroot)) (Transformation|GetWorldLocation _defaultsceneroot)) _returnvalue_3 (Utilities|Array|Get(acopy) (Variables|Default|GetDecals) (CallFunction|2DArrayIndexto1DIndex x y (.X (Utilities|Struct|BreakBP_2DArraysize_t (Variables|Default|GetspawnAmount)))))))

(fn GetDecalApproxPosition
  (params (x :type Float%20%28single-precision%29) (y :type Float%20%28single-precision%29))
  (bind _spawnevery (Variables|Default|GetspawnEvery))
  (bind _defaultsceneroot (Variables|Default|GetDefaultSceneRoot))
  (bind (_x _y) (Math|Vector2D|BreakVector2D _spawnevery))
  (bind _returnvalue (* _x x))
  (bind _returnvalue_2 (* _y y))
  (bind _returnvalue_3 (Math|Vector|MakeVector _returnvalue 0.0 _returnvalue_2))
  (return (+ (Transformation|GetWorldLocation _defaultsceneroot) (Math|Vector|RotateVector (* _returnvalue_3 (Transformation|GetWorldScale _defaultsceneroot)) (Transformation|GetWorldRotation _defaultsceneroot))) _returnvalue_3))