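; Decal-grid actor that projects text as a scrolling bitfont animation, playable a limited or unlimited number of times.
; PlayNewAnimation loads a data-table font, slices a canvas region from the decal grid, builds C++ BitString and BitCanvas objects, and caches decal materials and visibility for later restoration.
; Tick advances BitString, pushing each new column right to left into BitCanvas.
; Animation ticks and start, stop and pause callbacks are relayed as actor events.
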(event Custom|OnBitCanvasStarted
  ;[1 1 1] BitString Callback Events
  (Default|CallOnAnimationStart))

(event Custom|OnBitcanvasPaused
  ;[1 1 1] BitString Callback Events
  (Default|CallOnAnimationPaused))

(event Custom|OnAssignBitstringCalbacks
  (bind _bitstring (Variables|Default|GetbitString))
  ;[1 1 1] BitString Callback Events
  (EventDispatchers|AssignOnAnimationStart _bitstring (delegate Custom|OnBitCanvasStarted))
  (EventDispatchers|BindEventtoOnAnimationStop _bitstring (delegate Custom|OnBitCanvasStopped))
  (EventDispatchers|BindEventtoOnAnimationPause _bitstring (delegate Custom|OnBitcanvasPaused)))

(event Custom|OnBitCanvasStopped
  ;[1 1 1] BitString Callback Events
  (Default|CallOnAnimationStopped))

(event EventBeginPlay)

(event EventActorBeginOverlap
  (params (OtherActor :type Actor%20Object%20Reference)))

(event EventTick
  (params (DeltaSeconds :type Float%20%28single-precision%29))
  (bind _bitstring (Variables|Default|GetbitString))
  (bind _returnvalue (Class|AnimatedBitString|AnimationElapsed _bitstring true))
  (bind _returnvalue_2 (Class|AnimatedBitString|AnimationElapsedUnscaled _bitstring))
  (bind _returnvalue_3 (Class|BitfontFunctionLibrary|IsBitAnimationSafetoTick (Variables|Default|GetbitString) (Variables|Default|GetbitCanvas)))
  (if _returnvalue_3
    (bind (_outbuffer _returnvalue_4) (Class|AnimatedBitString|Tick (Variables|Default|GetbitString) DeltaSeconds))
    (Default|CallOnAnimationEnabled _returnvalue_2 _returnvalue)
    (if _returnvalue_4
      (Class|Bitcanvas|PushRighttoLeft (Variables|Default|GetbitCanvas) _outbuffer)
      (Default|CallOnAnimationTick _returnvalue_2 _returnvalue))))

(fn ConstructionScript
  (|CallParentFunction))

(fn CanvasWidth
  (bind _startcanvasatcolumn (Variables|Default|GetstartCanvasAtColumn))
  (bind _endcanvasatcolumn (Variables|Default|GetendCanvasAtColumn))
  (LocalVariables|SetA (Math|Integer|Min(Integer) _startcanvasatcolumn _endcanvasatcolumn))
  (LocalVariables|SetB (Math|Integer|Max(Integer) _startcanvasatcolumn _endcanvasatcolumn))
  (return (- (LocalVariables|GetB) (LocalVariables|GetA)) (LocalVariables|GetA)))

(fn PlayNewAnimation
  (params (text :type String%20%28by%20ref%29) (delaySeconds :type Float%20%28single-precision%29))
  (bind _playnoofanimations (Variables|Default|GetplayNoOfAnimations))
  (bind _bitcanvas (Variables|Default|GetbitCanvas))
  ;[1 1 1] Check max number of animations
  (if (or (== _playnoofanimations 0) (< (Variables|Default|GetanimationsPlayed) _playnoofanimations))
    (bind _returnvalue (Utilities|GetDataTableRow "/Game/Data/Bitfonts.Bitfonts" (Variables|Default|GetBitfontEntry))
      (:then
        ;[1 1 1] Initilaise C++ objects
        (bind (_outwidth _outheight) (CallFunction|FillCanvasDecalBuffer (LocalVariables|GetdecalBuffer) (.maxHeight (Utilities|Struct|BreakBitfont _returnvalue))))
        (Class|BitfontFunctionLibrary|BuildBitstringObjects _returnvalue (Variables|Default|GetbitString) text _bitcanvas (LocalVariables|GetdecalBuffer) _outwidth _outheight)
        (CallFunction|AssignBitstringCallbacks)
        (CallFunction|CacheMaterialPointers)
        (Class|Bitcanvas|AssignMaterial _bitcanvas (Variables|Default|GetstringMaterial))
        (Class|Bitcanvas|SetDisplayAll (Variables|Default|GetbitCanvas) false)
        ;[1 1 1] Start Animation
        (Class|AnimatedBitString|StartAfter (Variables|Default|GetbitString) (.width (CallFunction|CanvasWidth)) (Variables|Default|GettickAnimationEverySec) (Math|Float|Max(Float) delaySeconds 0.0))
        ;[1 1 1] Increment Animations Played
        (Variables|Default|SetanimationsPlayed (+ (Variables|Default|GetanimationsPlayed) 1))))))

(fn FillCanvasDecalBuffer
  (params (buffer :type Array%20of%20Decal%20Component%20Object%20References) (Height :type Integer))
  (bind (_width _firstvalue) (CallFunction|CanvasWidth))
  (Utilities|Array|Clear buffer)
  (LocalVariables|SetlocalHeight Height)
  (LocalVariables|SetlocalWidth _width)
  (LocalVariables|SetfirstColumn _firstvalue)
  (for _index (range 0 (- (LocalVariables|GetlocalHeight) 1))
    (for _index_2 (range 0 (- (LocalVariables|GetlocalWidth) 1))
      (Utilities|Array|Add buffer (Utilities|Array|Get(acopy) (Variables|Default|GetDecals) (+ (CallFunction|2DArrayIndexto1DIndex _index_2 (+ _index (Variables|Default|GetstartCanvasAtRow)) (.X (Utilities|Struct|BreakBP_2DArraysize_t (Variables|Default|GetspawnAmount)))) (LocalVariables|GetfirstColumn))))))
  (return (LocalVariables|GetlocalWidth) (LocalVariables|GetlocalHeight)))

(fn DisplayAllDecals
  (params (Display :type Boolean))
  (for _array_element (Variables|Default|GetDecals)
    (Rendering|SetVisibility _array_element Display false)))

(fn AssignBitstringCallbacks
  (if (!= (Variables|Default|GetbitString) 0)
    (CallFunction|OnAssignBitstringCalbacks)))

(fn CacheMaterialPointers
  (bind _decals (Variables|Default|GetDecals))
  (Utilities|Array|Clear (Variables|Default|GetDecalCache))
  (for _index (range 0 (- (Utilities|Array|Length _decals) 1))
    (Utilities|Array|Add (Variables|Default|GetDecalCache) (Utilities|Struct|MakeCachedDecal_t (Class|DecalComponent|GetDecalMaterial (Utilities|Array|Get(acopy) _decals _index)) (Rendering|IsVisible (Utilities|Array|Get(acopy) _decals _index))))))

(fn UnloadMaterialPointers
  (params (clearArray :type Boolean))
  (bind _decals (Variables|Default|GetDecals))
  (for _index (range 0 (- (Utilities|Array|Length _decals) 1))
    (Rendering|Components|Decal|SetDecalMaterial (Utilities|Array|Get(acopy) _decals _index) (.Material (Utilities|Struct|BreakCachedDecal_t (Utilities|Array|Get(acopy) (Variables|Default|GetDecalCache) _index))))
    (Rendering|SetVisibility (Utilities|Array|Get(acopy) _decals _index) (.Enabled (Utilities|Struct|BreakCachedDecal_t (Utilities|Array|Get(acopy) (Variables|Default|GetDecalCache) _index))) false))
  (if clearArray
    (Utilities|Array|Clear (Variables|Default|GetDecalCache))))

(fn AnimationFrames
  (if (!= (Variables|Default|GetbitString) 0)
    (return (Class|AnimatedBitString|TotalFrames (Variables|Default|GetbitString)))
    (else
      (return -1))))

(fn AnimationLength
  (bind _bitstring (Variables|Default|GetbitString))
  (if (!= _bitstring 0)
    (return (Class|AnimatedBitString|AnimationLength _bitstring))
    (else
      (return -1.0))))

(fn GetCanvasCenter
  (bind _bitcanvas (Variables|Default|GetbitCanvas))
  (bind (_x _y) (Class|Bitcanvas|GetCanvasCenter _bitcanvas))
  (Development|PrintString (Utilities|String|ToString(Float) _x))
  (if (!= _bitcanvas 0)
    (return (.position (CallFunction|GetDecalApproxPosition _x _y)))
    (else
      (return (Transformation|GetWorldLocation (Variables|Default|GetDefaultSceneRoot))))))