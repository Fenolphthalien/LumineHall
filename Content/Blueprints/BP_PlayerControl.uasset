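; Player controller that slides the BP_Player pawn along a spline from axis input and quits on Escape.
; Spline movement is gated by AllowInput, which blocks it during a timed lockout (paused while naming) or while the naming bar is open.
; Camera target transforms are passed to the pawn and blended through an animation curve on LumineHall ticks.
; A lazily created naming widget shows the player's name and saves edits when hidden.
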(event Custom|OnLumineHallTick
  (params (Time :type Float%20%28single-precision%29) (Scaled%20Time :type Float%20%28single-precision%29))
  (bind _asbp_player (Utilities|Casting|CastToBP_Player (Pawn|GetControlledPawn)))
  (bind _lerpedtransform (Default|LerpCameraTransform _asbp_player (Math|Curves|GetFloatValue (Variables|Default|GetanimationCurve) Scaled%20Time)))
  (Default|SetCamerafromTransform _asbp_player _lerpedtransform))

(event EventTick
  (params (DeltaSeconds :type Float%20%28single-precision%29))
  (if (not (CallFunction|AllowInput))
    (if (not (Variables|Default|GetDrawingNamingWidget))
      (Variables|Default|SetpreventInputWait (- (Variables|Default|GetpreventInputWait) DeltaSeconds)))))

(event Input|AxisEvents|InputAxisMoveAlongSpline
  (params (AxisValue :type Float%20%28single-precision%29))
  (bind _spline (Variables|Default|GetSpline))
  (if (CallFunction|AllowInput)
    (Variables|Default|SetdistanceTraveled (+ (Variables|Default|GetdistanceTraveled) (* AxisValue (* (Variables|Default|Getspeed) (Utilities|Time|GetWorldDeltaSeconds)))))
    (if (!= _spline 0)
      (Transformation|SetActorLocation (Pawn|GetControlledPawn) (Spline|GetLocationatDistanceAlongSpline _spline (Variables|Default|GetdistanceTraveled) "World") false false))))

(event Input|KeyboardEvents|Escape
  (params (Key :type Key%20Structure :default "AnyKey"))
  (:Pressed
    (Game|QuitGame self "Quit")))

(fn ConstructionScript)

(fn PreventInputfor
  (params (seconds :type Float%20%28single-precision%29) (OverrideExistingWait :type Boolean))
  (if (and (> seconds 0.0) (or OverrideExistingWait (> seconds (Variables|Default|GetpreventInputWait))))
    (Variables|Default|SetpreventInputWait seconds))
  (return))

(fn AllowInput
  (return (and (not (> (Variables|Default|GetpreventInputWait) 0.0)) (not (Variables|Default|GetDrawingNamingWidget)))))

(fn ForceRegainControl
  (Variables|Default|SetpreventInputWait 0.0))

(fn SetCameraTarget
  (params (transform :type Camera%20Transform%20Structure))
  (bind _asbp_player (Utilities|Casting|CastToBP_Player (Pawn|GetControlledPawn)))
  (Variables|/Game/Blueprints/BP_Player.BP_Player_C|SetcameraTransformTarget _asbp_player transform))

(fn SetCameraTargetfromWorld
  (params (TargetPosition :type Vector) (Rotation :type Rotator) (Distance :type Float%20%28single-precision%29) (FOV :type Float%20%28single-precision%29))
  (CallFunction|SetCameraTarget (Utilities|Struct|MakeCameraTransform TargetPosition Rotation Distance FOV)))

(fn ToggleNamingBar
  (bind _returnvalue (Pawn|GetControlledPawn))
  (bind _output_get (Variables|Default|SetDrawingNamingWidget (not (Variables|Default|GetDrawingNamingWidget))))
  (if _output_get
    (if (== (Variables|Default|GetnamingBar) 0)
      (bind _returnvalue_2 (UserInterface|CreateWidget "/Game/Blueprints/Widgets/NamingBar.NamingBar_C" self))
      (Variables|Default|SetnamingBar _returnvalue_2)
      (UserInterface|Viewport|AddtoViewport (Variables|Default|GetnamingBar) 0))
    (Widget|SetVisibility (Variables|Default|GetnamingBar) "Visible")
    (bind _asbp_player (Utilities|Casting|CastToBP_Player _returnvalue))
    (bind _name (Default|GetName _asbp_player))
    (Default|SetText (Variables|Default|GetnamingBar) (Utilities|Text|ToText(String) _name))
    (else
      (Widget|SetVisibility (Variables|Default|GetnamingBar) "Hidden")
      (bind _asbp_player_2 (Utilities|Casting|CastToBP_Player _returnvalue))
      (Default|SetName _asbp_player_2 (Utilities|String|ToString(Text) (Default|GetText0 (Variables|Default|GetnamingBar)))))))