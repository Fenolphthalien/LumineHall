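; Player Blueprint that manages a pivot-based camera rig and exposes the character's name.
; On BeginPlay it captures the pivot's relative location and rotation, the camera's X distance and FOV as both default and target camera transform.
; Helper functions interpolate from default to target by an alpha, using shortest-path rotation, and apply a transform to the rig.
; Nothing in this graph calls the interpolation or apply helpers.
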(event EventBeginPlay
  (bind _transform (CallFunction|MakeCameraTransform))
  (bind _output_get (Variables|Default|SetDefaultCameraTransform _transform))
  (Variables|Default|SetcameraTransformTarget _output_get))

(event EventActorBeginOverlap
  (params (OtherActor :type Actor%20Object%20Reference)))

(event EventTick
  (params (DeltaSeconds :type Float%20%28single-precision%29)))

(fn ConstructionScript)

(fn MakeCameraTransform
  (bind _camera (Variables|Default|GetCamera))
  (bind _camera_pivot (Variables|Default|GetCamera%20Pivot))
  (return (Utilities|Struct|MakeCameraTransform (Variables|/Script/Engine.SceneComponent|GetRelativeLocation _camera_pivot) (Variables|/Script/Engine.SceneComponent|GetRelativeRotation _camera_pivot) (.X (Math|Vector|BreakVector (Variables|/Script/Engine.SceneComponent|GetRelativeLocation _camera))) (Variables|/Script/Engine.CameraComponent|GetFieldOfView _camera))))

(fn LerpCameraTransform
  (params (Value :type Float%20%28single-precision%29))
  (bind _defaultcameratransform (Variables|Default|GetDefaultCameraTransform))
  (bind _cameratransformtarget (Variables|Default|GetcameraTransformTarget))
  (bind (_position _rotation _distance _fov) (Utilities|Struct|BreakCameraTransform _cameratransformtarget))
  (bind (_position_2 _rotation_2 _distance_2 _fov_2) (Utilities|Struct|BreakCameraTransform _defaultcameratransform))
  (return (Utilities|Struct|MakeCameraTransform (Math|Vector|Lerp(Vector) _position_2 _position Value) (Math|Rotator|Lerp(Rotator) _rotation_2 _rotation Value true) (Math|Float|Lerp _distance_2 _distance Value) (Math|Float|Lerp _fov_2 _fov Value))))

(fn SetCamerafromTransform
  (params (transform :type Camera%20Transform%20Structure%20%28by%20ref%29))
  (bind (_position _rotation _distance _fov) (Utilities|Struct|BreakCameraTransform transform))
  (bind _camera_pivot (Variables|Default|GetCamera%20Pivot))
  (bind _camera (Variables|Default|GetCamera))
  (Transformation|SetRelativeRotation _camera_pivot _rotation false false)
  (Transformation|SetRelativeLocation _camera_pivot _position false false)
  (Transformation|SetRelativeLocation _camera (Math|Vector|MakeVector _distance 0.0 0.0) false false)
  (Variables|/Script/Engine.CameraComponent|SetFieldOfView _camera _fov))

(fn GetName
  (return (Variables|Default|GetCharacterName)))